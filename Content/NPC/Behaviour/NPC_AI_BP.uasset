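; AI controller for guard NPCs that patrol and open fire on perceived targets.
; On begin play it loads the patrol blackboard, runs the guard behavior tree and caches its pawn as TPCharacter.
; AI Perception updates respond only to actors without the "Enemy" tag.
; Sensing one writes it to the blackboard and turns on the pawn's aiming and shooting; losing it clears both.
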(event OnTargetPerceptionUpdated(AIPerception)
  (params (Actor :type Actor%20Object%20Reference) (Stimulus :type AI%20Stimulus%20Structure))
  (bind _blackboardcomp (Variables|Default|GetBlackboardComp))
  (bind _enemykey (Variables|Default|GetEnemyKey))
  (if (not (Actor|ActorHasTag Actor "Enemy"))
    (if (.bSuccessfullySensed (Utilities|Struct|BreakAIStimulus Stimulus))
      (AI|Components|Blackboard|SetValueasObject _blackboardcomp _enemykey Actor)
      (Variables|/Game/NPC/Behaviour/TPCharacter.TPCharacter_C|SetAiming (stale EventBeginPlay _astpcharacter) true)
      (Variables|/Game/NPC/Behaviour/TPCharacter.TPCharacter_C|SetShooting (stale EventBeginPlay _astpcharacter) true)
      (else
        (AI|Components|Blackboard|ClearValue _blackboardcomp _enemykey)
        (Variables|/Game/NPC/Behaviour/TPCharacter.TPCharacter_C|SetAiming (stale EventBeginPlay _astpcharacter) false)
        (Variables|/Game/NPC/Behaviour/TPCharacter.TPCharacter_C|SetShooting (stale EventBeginPlay _astpcharacter) false)))))

(event EventBeginPlay
  (bind _blackboardcomponent (Class|AIController|UseBlackboard "/Game/NPC/Behaviour/PatrolData.PatrolData"))
  (Variables|Default|SetBlackboardComp _blackboardcomponent)
  (AI|RunBehaviorTree "/Game/NPC/Behaviour/GuardBehaviour.GuardBehaviour")
  (bind _astpcharacter (Utilities|Casting|CastToTPCharacter (Pawn|GetControlledPawn))))

(fn ConstructionScript)